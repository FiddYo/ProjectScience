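; Inventory component from the CompoundCreator folder that stores items as a map of item names to integer quantities.
; Adding stacks onto any existing count, while removal fails when the stock is insufficient and deletes entries that reach zero.
; Swapping is a one-way transfer that adds the items to a target inventory only if removal from this one succeeds.
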(event EventBeginPlay)

(event EventTick
  (params (DeltaSeconds :type Float%20%28single-precision%29)))

(fn BPAddtoInventory
  (params (ItemName :type Name) (Quantity :type Integer))
  (bind _inventorycontent (Variables|Default|GetInventoryContent))
  (bind (_value _returnvalue) (Utilities|Map|Find _inventorycontent ItemName))
  (Utilities|Map|Add _inventorycontent ItemName (Math|Integer|SelectInt (+ Quantity _value) Quantity _returnvalue)))

(fn BPRemovefromInventory
  (params (ItemName :type Name) (Quantity :type Integer))
  (bind _inventorycontent (Variables|Default|GetInventoryContent))
  (bind _value (Utilities|Map|Find _inventorycontent ItemName))
  (bind _returnvalue (- _value Quantity))
  (if (<= Quantity _value)
    (if (== _returnvalue 0)
      (Utilities|Map|Remove (Variables|Default|GetInventoryContent) ItemName)
      (return true)
      (else
        (Utilities|Map|Add (Variables|Default|GetInventoryContent) ItemName _returnvalue)
        (return true)))
    (else
      (return false))))

(fn BPSwapwithInventory
  (params (TargetInventory :type BP%20Inventory%20Component%20Object%20Reference) (ItemName :type Name) (Quantity :type Integer))
  (bind _success (CallFunction|RemovefromInventory ItemName Quantity))
  (if _success
    (CallFunction|AddtoInventory TargetInventory ItemName Quantity)))