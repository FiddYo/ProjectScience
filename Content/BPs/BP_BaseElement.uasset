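; BP_BaseElement displays a chemical element as an atom through a Niagara particle system.
; NewFunction0 feeds proton, neutron and electron counts into Niagara spawn parameters, reinitializing the system after each change.
; It derives sphere radius from the atomic number, doubled for the lightest elements and capped.
; The construction script is empty, leaving disconnected draft logic that queries WBP_Chemistry widgets and sets the same parameters.
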(fn ConstructionScript)

(fn NewFunction0
  (params (NewParam :type Element%20Structure%20Structure) (Protons :type Integer) (Neutrons :type Integer) (Electrons :type Integer))
  (bind _atomicnumber (Utilities|Struct|BreakElementStructure NewParam))
  (Utilities|FlowControl|Sequence
    (:then_0
      (if (< _atomicnumber 6)
        (Variables|Default|SetinValue (Math|Conversions|ToFloat(Integer) (* _atomicnumber 2)))
        (else
          (Variables|Default|SetinValue (Math|Conversions|ToFloat(Integer) _atomicnumber))))
      (Niagara|SetNiagaraVariable(Float) (Variables|Default|GetNiagara) "SphereRadius" (Math|Float|Min(Float) (Variables|Default|GetinValue) 3e+01)))
    (:then_1
      (Niagara|SetNiagaraVariable(Float) (Variables|Default|GetNiagara) "SpawnCountProtons" (Math|Conversions|ToFloat(Integer) Protons)))
    (:then_2
      (Niagara|SetNiagaraVariable(Float) (Variables|Default|GetNiagara) "SpawnCountNeutrons" (Math|Conversions|ToFloat(Integer) Neutrons)))
    (:then_3
      (Niagara|SetNiagaraVariable(Float) (Variables|Default|GetNiagara) "SpawnCountElectrons" (Math|Conversions|ToFloat(Integer) Electrons))))
  (Niagara|ReinitializeSystem (Variables|Default|GetNiagara)))