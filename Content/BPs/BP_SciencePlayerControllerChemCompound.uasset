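; Player controller for a chemistry compound science game, handling camera views, cursor toggling and the pause menu.
; The mouse wheel steps between primary camera actor, secondary self view and a hovered interactable's child camera via blended view targets, blocked while the HUD inventory is open, except secondary-to-primary.
; Zooming in requires a cursor hit.
; FlipFlops drive Left Alt's cursor toggle and Tab's cached pause widget.
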(event Input|KeyboardEvents|Tab
  (params (Key :type Key%20Structure :default "None"))
  (:Pressed
    (Utilities|FlowControl|FlipFlop
      (:A
        (bind _pausemenuref (Variables|Default|GetPauseMenuRef)
          (:then
            (UserInterface|Viewport|AddtoViewport _pausemenuref 0))
          (:else
            (bind _returnvalue (UserInterface|CreateWidget "/Game/UI/WBPs/WBP_Pause.WBP_Pause_C"))
            (bind _output_get (Variables|Default|SetPauseMenuRef _returnvalue))
            (UserInterface|Viewport|AddtoViewport _output_get 0)
            (Variables|/Script/Engine.PlayerController|SetbShowMouseCursor (Game|GetPlayerController 0) true))))
      (:B
        (bind _pausemenuref_2 (Variables|Default|GetPauseMenuRef)
          (:then
            (Widget|RemovefromParent _pausemenuref_2))
          (:else))))))

(event Input|MouseEvents|MouseWheelUp
  (params (Key :type Key%20Structure :default "None"))
  (bind _returnvalue (Game|GetPlayerController 0))
  (bind _array (Utilities|Array|MakeArray "ObjectTypeQuery1" "ObjectTypeQuery2" "ObjectTypeQuery3" "ObjectTypeQuery4" "ObjectTypeQuery5" "ObjectTypeQuery6"))
  (bind (_hitresult _returnvalue_2) (Class|PlayerController|GetHitResultUnderCursorforObjects _returnvalue _array true))
  (:Pressed
    (bind _open_ (CallFunction|CheckInventoryOpen))
    (if (and (not _open_) _returnvalue_2)
      (if (Variables|Default|GetbPrimary)
        (CallFunction|SetSecondaryView)
        (elif (Variables|Default|GetbSecondary)
          (CallFunction|SetTertiaryView (.HitActor (Collision|BreakHitResult _hitresult))))))))

(event Input|MouseEvents|MouseWheelDown
  (params (Key :type Key%20Structure :default "None"))
  (:Pressed
    (bind _open_ (CallFunction|CheckInventoryOpen))
    (if (and (not _open_) (Variables|Default|GetbTertiary))
      (CallFunction|SetSecondaryView)
      (elif (Variables|Default|GetbSecondary)
        (CallFunction|SetPrimaryView)))))

(event Input|KeyboardEvents|LeftAlt
  (params (Key :type Key%20Structure :default "None"))
  (:Pressed
    (bind _isa (Utilities|FlowControl|FlipFlop)
      (:A
        (Variables|Default|SetbShowMouseCursor _isa))
      (:B
        (Variables|Default|SetbShowMouseCursor _isa)))))

(fn ConstructionScript)

(fn BPSetSecondaryView
  (Game|Player|SetViewTargetwithBlend self 0.5 "VTBlend_Linear" 1.0 true)
  (Variables|Default|SetbTertiary false)
  (Variables|Default|SetbSecondary true)
  (Variables|Default|SetbPrimary false))

(fn BPSetTertiaryView
  (params (Object :type Object%20Object%20Reference))
  (bind _asbp_base_interactable (Utilities|Casting|CastToBP_BaseInteractable Object))
  (Game|Player|SetViewTargetwithBlend (Variables|/Script/Engine.ChildActorComponent|GetChildActor (Variables|/Game/BPs/BP_BaseInteractable.BP_BaseInteractable_C|GetBP_cameraActor _asbp_base_interactable)) 0.5 "VTBlend_Linear" 0.0 true)
  (Variables|Default|SetbTertiary true)
  (Variables|Default|SetbSecondary false)
  (Variables|Default|SetbPrimary false))

(fn BPSetPrimaryView
  (bind _returnvalue (Actor|GetActorOfClass "/Game/BPs/BP_cameraActorPrimary.BP_cameraActorPrimary_C"))
  (Game|Player|SetViewTargetwithBlend _returnvalue 0.5 "VTBlend_Linear" 0.0 true)
  (Variables|Default|SetbTertiary false)
  (Variables|Default|SetbSecondary false)
  (Variables|Default|SetbPrimary true))

(fn BPCheckInventoryOpen
  (bind _asbp_science_hud (Utilities|Casting|CastToBP_ChemCompoundHUD (HUD|GetHUD)))
  (return (Variables|/Game/UI/WBPs/WBP_HUDCompoundCreator.WBP_HUDCompoundCreator_C|GetbInventoryOpen (Variables|/Game/BPs/BP_ChemCompoundHUD.BP_ChemCompoundHUD_C|GetHudWidgetRef _asbp_science_hud))))