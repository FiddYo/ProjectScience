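; Game mode for the science compound-creation game that fills the order screen with randomly picked orders.
; BeginPlay calls GenerateNewOrder a random number of times.
; BPGenerateNewOrder picks a random OrderDataTable row and adds an entry widget to BP_OrderScreen's UI, showing name, days, difficulty-scaled cash, instructions and icons.
; Completion requirements are balanced across the entry's left and right scroll boxes.
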(event EventBeginPlay
  (bind _returnvalue (Math|Random|RandomIntegerinRange 0 5))
  (Variables|Default|Setrandom _returnvalue)
  (Development|PrintString (Utilities|String|ToString(Integer) (Variables|Default|Getrandom)))
  (for _index (range 0 _returnvalue)
    (CallFunction|GenerateNewOrder)))

(fn ConstructionScript)

(fn BPGenerateNewOrder
  (bind _returnvalue (Actor|GetActorOfClass "/Game/BPs/CompoundCreator/BP_OrderScreen.BP_OrderScreen_C"))
  (bind _aswbp_order_screen_ui (Utilities|Casting|CastToWBP_OrderScreenUI (UserInterface|GetWidget (Variables|/Game/BPs/CompoundCreator/BP_OrderScreen.BP_OrderScreen_C|GetWidget_0 _returnvalue))))
  (bind _returnvalue_2 (UserInterface|CreateWidget "/Game/UI/WBPs/CompoundCreator/WBP_OrderEntryNew.WBP_OrderEntryNew_C"))
  (bind _outrownames (DataTable|GetDataTableRowNames "/Game/Data/CompoundCreator/OrderDataTable.OrderDataTable"))
  (bind _returnvalue_3 (Utilities|GetDataTableRow "/Game/Data/CompoundCreator/OrderDataTable.OrderDataTable" (Utilities|Array|Get(acopy) _outrownames (Math|Random|RandomIntegerinRange 0 (Utilities|Array|Length _outrownames))))
    (:then
      (Variables|/Game/UI/WBPs/CompoundCreator/WBP_OrderEntryNew.WBP_OrderEntryNew_C|SetOrderData _returnvalue_2 _returnvalue_3)
      (Rendering|Components|TextRender|SetText (Variables|/Game/UI/WBPs/CompoundCreator/WBP_OrderEntryExpansionHead.WBP_OrderEntryExpansionHead_C|GetOrdernameText (Variables|/Game/UI/WBPs/CompoundCreator/WBP_OrderEntryNew.WBP_OrderEntryNew_C|GetWBP_OrderEntryExpansionHeadNew _returnvalue_2)) (Utilities|Text|ToText(String) (.OrderName (Utilities|Struct|BreakOrderDataStruct _returnvalue_3))))
      (switch Utilities|FlowControl|Switch|SwitchonOrderDifficultyEnum (.Difficulty (Utilities|Struct|BreakOrderDataStruct _returnvalue_3))
        (:NewEnumerator0
          (LocalVariables|SetDifficultyMultiplier 2.0))
        (:NewEnumerator1
          (LocalVariables|SetDifficultyMultiplier 3.0))
        (:NewEnumerator2
          (LocalVariables|SetDifficultyMultiplier 4.0)))
      (Rendering|Components|TextRender|SetText (Variables|/Game/UI/WBPs/CompoundCreator/WBP_OrderEntryExpansionHead.WBP_OrderEntryExpansionHead_C|GetDaysRewardText (Variables|/Game/UI/WBPs/CompoundCreator/WBP_OrderEntryNew.WBP_OrderEntryNew_C|GetWBP_OrderEntryExpansionHeadNew _returnvalue_2)) (Utilities|Text|FormatText "{days}Days 
${cash}" (.Days (Utilities|Struct|BreakOrderDataStruct _returnvalue_3)) (Math|Float|Truncate (* (.Cash (Utilities|Struct|BreakOrderDataStruct _returnvalue_3)) (LocalVariables|GetDifficultyMultiplier)))))
      (Rendering|Components|TextRender|SetText (Variables|/Game/UI/WBPs/CompoundCreator/WBP_OrderEntryExpansionNew.WBP_OrderEntryExpansionNew_C|GetInstructionTextNew (Variables|/Game/UI/WBPs/CompoundCreator/WBP_OrderEntryNew.WBP_OrderEntryNew_C|GetWBP_OrderEntryExpansionNew _returnvalue_2)) (Utilities|Text|ToText(String) (.InstructionText (Utilities|Struct|BreakOrderDataStruct _returnvalue_3))))
      (for _array_element (.Icon (Utilities|Struct|BreakOrderDataStruct _returnvalue_3))
        (bind _returnvalue_4 (UserInterface|CreateWidget "/Game/UI/WBPs/CompoundCreator/WBP_IconScaleBox.WBP_IconScaleBox_C"))
        (Class|Image|SetBrush (Variables|/Game/UI/WBPs/CompoundCreator/WBP_IconScaleBox.WBP_IconScaleBox_C|GetIcon _returnvalue_4) (Utilities|Struct|MakeSlateBrush (.ImageSize (Utilities|Struct|BreakSlateBrush (Variables|/Script/UMG.Image|GetBrush (Variables|/Game/UI/WBPs/CompoundCreator/WBP_IconScaleBox.WBP_IconScaleBox_C|GetIcon _returnvalue_4)))) (.Margin (Utilities|Struct|BreakSlateBrush (Variables|/Script/UMG.Image|GetBrush (Variables|/Game/UI/WBPs/CompoundCreator/WBP_IconScaleBox.WBP_IconScaleBox_C|GetIcon _returnvalue_4)))) (.TintColor (Utilities|Struct|BreakSlateBrush (Variables|/Script/UMG.Image|GetBrush (Variables|/Game/UI/WBPs/CompoundCreator/WBP_IconScaleBox.WBP_IconScaleBox_C|GetIcon _returnvalue_4)))) (.OutlineSettings (Utilities|Struct|BreakSlateBrush (Variables|/Script/UMG.Image|GetBrush (Variables|/Game/UI/WBPs/CompoundCreator/WBP_IconScaleBox.WBP_IconScaleBox_C|GetIcon _returnvalue_4)))) _array_element (.DrawAs (Utilities|Struct|BreakSlateBrush (Variables|/Script/UMG.Image|GetBrush (Variables|/Game/UI/WBPs/CompoundCreator/WBP_IconScaleBox.WBP_IconScaleBox_C|GetIcon _returnvalue_4)))) (.Tiling (Utilities|Struct|BreakSlateBrush (Variables|/Script/UMG.Image|GetBrush (Variables|/Game/UI/WBPs/CompoundCreator/WBP_IconScaleBox.WBP_IconScaleBox_C|GetIcon _returnvalue_4)))) (.Mirroring (Utilities|Struct|BreakSlateBrush (Variables|/Script/UMG.Image|GetBrush (Variables|/Game/UI/WBPs/CompoundCreator/WBP_IconScaleBox.WBP_IconScaleBox_C|GetIcon _returnvalue_4))))))
        (Widget|Panel|AddChild (Variables|/Game/UI/WBPs/CompoundCreator/WBP_OrderEntryExpansionHead.WBP_OrderEntryExpansionHead_C|GetTextAndIconHolder (Variables|/Game/UI/WBPs/CompoundCreator/WBP_OrderEntryNew.WBP_OrderEntryNew_C|GetWBP_OrderEntryExpansionHeadNew _returnvalue_2)) _returnvalue_4))
      (for _array_element_2 (.CompletionRequirements (Utilities|Struct|BreakOrderDataStruct _returnvalue_3))
        (bind _returnvalue_5 (UserInterface|CreateWidget "/Game/UI/WBPs/CompoundCreator/WBP_CompletionRequirementText.WBP_CompletionRequirementText_C"))
        (Rendering|Components|TextRender|SetText (Variables|/Game/UI/WBPs/CompoundCreator/WBP_CompletionRequirementText.WBP_CompletionRequirementText_C|GetText _returnvalue_5) (Utilities|Text|FormatText "{Quant} x {Name}" (.Quantity (Utilities|Struct|BreakCompletionRequirementsStruct _array_element_2)) (.Name (Utilities|Struct|BreakCompletionRequirementsStruct _array_element_2))))
        (if (> (Utilities|Array|Length (Class|PanelWidget|GetAllChildren (Variables|/Game/UI/WBPs/CompoundCreator/WBP_OrderEntryExpansionNew.WBP_OrderEntryExpansionNew_C|GetLeftScrollBox (Variables|/Game/UI/WBPs/CompoundCreator/WBP_OrderEntryNew.WBP_OrderEntryNew_C|GetWBP_OrderEntryExpansionNew _returnvalue_2)))) (Utilities|Array|Length (Class|PanelWidget|GetAllChildren (Variables|/Game/UI/WBPs/CompoundCreator/WBP_OrderEntryExpansionNew.WBP_OrderEntryExpansionNew_C|GetRightScrollBox (Variables|/Game/UI/WBPs/CompoundCreator/WBP_OrderEntryNew.WBP_OrderEntryNew_C|GetWBP_OrderEntryExpansionNew _returnvalue_2)))))
          (Widget|Panel|AddChild (Variables|/Game/UI/WBPs/CompoundCreator/WBP_OrderEntryExpansionNew.WBP_OrderEntryExpansionNew_C|GetRightScrollBox (Variables|/Game/UI/WBPs/CompoundCreator/WBP_OrderEntryNew.WBP_OrderEntryNew_C|GetWBP_OrderEntryExpansionNew _returnvalue_2)) _returnvalue_5)
          (else
            (Widget|Panel|AddChild (Variables|/Game/UI/WBPs/CompoundCreator/WBP_OrderEntryExpansionNew.WBP_OrderEntryExpansionNew_C|GetLeftScrollBox (Variables|/Game/UI/WBPs/CompoundCreator/WBP_OrderEntryNew.WBP_OrderEntryNew_C|GetWBP_OrderEntryExpansionNew _returnvalue_2)) _returnvalue_5))))
      (Widget|Panel|AddChild (Variables|/Game/UI/WBPs/CompoundCreator/WBP_OrderScreenUI.WBP_OrderScreenUI_C|GetLeftScrollBoxNew _aswbp_order_screen_ui) _returnvalue_2))
    (:RowNotFound
      (Development|PrintString "data table not found"))))