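; Rack insert actor for the Compound Creator packing station, with a function meant to set child actor classes.
; BPSetChildClass takes a parameter but has an empty body, and the construction script is also empty.
; An unconnected chain of three nested checks compares ChildActor to the parameter before calling SetChildActorClass, so that logic never runs.
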(fn ConstructionScript)

(fn BPSetChildClass
  (params (NewParam :type Actor%20Object%20Reference)))