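; Packing station actor where clicking rack and shelf items assembles a compound in a packing slot: shell, then insert, then lid.
; BeginPlay binds click events on the child actors of the shell rack, insert rack and two lid shelves.
; Placement flags gate the order; each click sets the matching slot mesh, with inserts and lids eased into position by MoveComponentTo.
; Clicked items are hidden and reappear after a short delay to refill the racks.
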(event Custom|ClickBase
  (params (TouchedActor :type Actor%20Object%20Reference) (ButtonPressed :type Key%20Structure :default "None"))
  (if (Math|Boolean|ANDBoolean (not (Variables|Default|GetbHasPlacedLid)) (not (Variables|Default|GetbHasPlacedBase)) (not (Variables|Default|GetbHasPlacedInsert)))
    (bind _asbp_packing_slot_actor (Utilities|Casting|CastToBP_PackingSlotActor (Variables|/Script/Engine.ChildActorComponent|GetChildActor (Variables|Default|GetBP_PackingSlotActor))))
    (Components|StaticMesh|SetStaticMesh (Variables|/Game/BPs/CompoundCreator/PackingStation/BP_PackingSlotActor.BP_PackingSlotActor_C|GetShell _asbp_packing_slot_actor) "/Game/InteriorLaboratory/Meshes/SM_Bowl_01.SM_Bowl_01")
    (Utilities|Array|AddUnique (Variables|Default|GetShells) TouchedActor)
    (Rendering|SetActorHiddenInGame TouchedActor true)
    (Utilities|FlowControl|Delay 2.0)
    (for _array_element (Variables|Default|GetShells)
      (Rendering|SetActorHiddenInGame _array_element false)
      (Variables|Default|SetbHasPlacedBase true))))

(event Custom|ClickedInsert
  (params (TouchedActor :type Actor%20Object%20Reference) (ButtonPressed :type Key%20Structure :default "None"))
  (if (and (not (Variables|Default|GetbHasPlacedLid)) (Variables|Default|GetbHasPlacedBase))
    (Utilities|FlowControl|Sequence
      (:then_0
        (Utilities|Array|AddUnique (Variables|Default|GetInserts) TouchedActor)
        (Rendering|SetActorHiddenInGame TouchedActor true)
        (Variables|Default|SetbHasPlacedInsert true)
        (Utilities|FlowControl|Delay 2.0)
        (CallFunction|RefillInserts))
      (:then_1
        (bind _asbp_packing_slot_actor (Utilities|Casting|CastToBP_PackingSlotActor (Variables|/Script/Engine.ChildActorComponent|GetChildActor (Variables|Default|GetBP_PackingSlotActor))))
        (Components|StaticMesh|SetStaticMesh (Variables|/Game/BPs/CompoundCreator/PackingStation/BP_PackingSlotActor.BP_PackingSlotActor_C|GetInsert _asbp_packing_slot_actor) "/Game/InteriorLaboratory/Meshes/SM_Bowl_01.SM_Bowl_01")
        (Rendering|SetVisibility (Variables|/Game/BPs/CompoundCreator/PackingStation/BP_PackingSlotActor.BP_PackingSlotActor_C|GetInsert _asbp_packing_slot_actor) true false)
        (Components|MoveComponentTo (Variables|/Game/BPs/CompoundCreator/PackingStation/BP_PackingSlotActor.BP_PackingSlotActor_C|GetInsert _asbp_packing_slot_actor) (Variables|/Script/Engine.SceneComponent|GetRelativeLocation (Variables|/Game/BPs/CompoundCreator/PackingStation/BP_PackingSlotActor.BP_PackingSlotActor_C|GetShell _asbp_packing_slot_actor)) (Variables|/Script/Engine.SceneComponent|GetRelativeRotation (Variables|/Game/BPs/CompoundCreator/PackingStation/BP_PackingSlotActor.BP_PackingSlotActor_C|GetShell _asbp_packing_slot_actor)) false true 1.0 false)))))

(event Custom|ClickedLid
  (params (TouchedActor :type Actor%20Object%20Reference) (ButtonPressed :type Key%20Structure :default "None"))
  (if (and (Variables|Default|GetbHasPlacedBase) (Variables|Default|GetbHasPlacedInsert))
    (if (not (Variables|/Script/Engine.Actor|GetbHidden TouchedActor))
      (bind _asbp_packing_slot_actor (Utilities|Casting|CastToBP_PackingSlotActor (Variables|/Script/Engine.ChildActorComponent|GetChildActor (Variables|Default|GetBP_PackingSlotActor))))
      (Utilities|FlowControl|Sequence
        (:then_0
          (Utilities|Array|AddUnique (Variables|Default|GetLids) TouchedActor)
          (Rendering|SetActorHiddenInGame TouchedActor true)
          (Variables|Default|SetbHasPlacedLid true)
          (Utilities|FlowControl|Delay 2.0)
          (CallFunction|RefillLids))
        (:then_1
          (Components|StaticMesh|SetStaticMesh (Variables|/Game/BPs/CompoundCreator/PackingStation/BP_PackingSlotActor.BP_PackingSlotActor_C|GetLid _asbp_packing_slot_actor) "/Game/StarterContent/Shapes/Shape_NarrowCapsule.Shape_NarrowCapsule")
          (Rendering|SetVisibility (Variables|/Game/BPs/CompoundCreator/PackingStation/BP_PackingSlotActor.BP_PackingSlotActor_C|GetLid _asbp_packing_slot_actor) true false)
          (Components|MoveComponentTo (Variables|/Game/BPs/CompoundCreator/PackingStation/BP_PackingSlotActor.BP_PackingSlotActor_C|GetLid _asbp_packing_slot_actor) (+ (Variables|/Script/Engine.SceneComponent|GetRelativeLocation (Variables|/Game/BPs/CompoundCreator/PackingStation/BP_PackingSlotActor.BP_PackingSlotActor_C|GetShell _asbp_packing_slot_actor)) "0,0,35.000000") (Variables|/Script/Engine.SceneComponent|GetRelativeRotation (Variables|/Game/BPs/CompoundCreator/PackingStation/BP_PackingSlotActor.BP_PackingSlotActor_C|GetShell _asbp_packing_slot_actor)) false true 1.0 false))))))

(event EventBeginPlay
  (bind _bp_rackactor (Variables|Default|GetBP_RackActor))
  (bind _childactor (Variables|/Script/Engine.ChildActorComponent|GetChildActor _bp_rackactor))
  (bind _asbp_rack_actor_shells (Utilities|Casting|CastToBP_RackActorShells _childactor))
  (EventDispatchers|BindEventtoOnClicked _childactor (delegate Custom|ClickBase))
  (bind _asbp_rack_actor_inserts (Utilities|Casting|CastToBP_RackActorInserts (Variables|/Script/Engine.ChildActorComponent|GetChildActor (Variables|Default|GetBP_RackActorInserts))))
  (EventDispatchers|BindEventtoOnClicked (Variables|/Script/Engine.ChildActorComponent|GetChildActor (Variables|/Game/BPs/CompoundCreator/PackingStation/BP_RackActorInserts.BP_RackActorInserts_C|GetBP_InsertActor1 _asbp_rack_actor_inserts)) (delegate Custom|ClickedInsert))
  (bind _asbp_shelf_actor (Utilities|Casting|CastToBP_ShelfActor (Variables|/Script/Engine.ChildActorComponent|GetChildActor (Variables|Default|GetBP_ShelfActorLeft))))
  (EventDispatchers|BindEventtoOnClicked (Variables|/Script/Engine.ChildActorComponent|GetChildActor (Variables|/Game/BPs/CompoundCreator/PackingStation/BP_ShelfActor.BP_ShelfActor_C|GetBP_LidActor _asbp_shelf_actor)) (delegate Custom|ClickedLid))
  (bind _asbp_shelf_actor_2 (Utilities|Casting|CastToBP_ShelfActor (Variables|/Script/Engine.ChildActorComponent|GetChildActor (Variables|Default|GetBP_ShelfActorRight))))
  (EventDispatchers|BindEventtoOnClicked (Variables|/Script/Engine.ChildActorComponent|GetChildActor (Variables|/Game/BPs/CompoundCreator/PackingStation/BP_ShelfActor.BP_ShelfActor_C|GetBP_LidActor _asbp_shelf_actor_2)) (delegate Custom|ClickedLid)))

(fn ConstructionScript)

(fn BPRefillLids
  (for _array_element (Variables|Default|GetLids)
    (Rendering|SetActorHiddenInGame _array_element false)))

(fn BPRefillInserts
  (for _array_element (Variables|Default|GetInserts)
    (Rendering|SetActorHiddenInGame _array_element false)))