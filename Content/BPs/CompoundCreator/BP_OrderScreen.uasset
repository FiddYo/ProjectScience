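; Order screen actor for the compound-creator game that tracks the player's average star rating across orders and pays out order cash.
; BP_CalculateStarRating averages each incoming rating with past ones, snapping near-perfect averages to five on a five-star order, and adds cash to BP_ScienceGameModeCompCreate.
; It updates the widget's star progress bar and mirrors state into RatingStruct, which BP_LoadValuesFromSave uses to restore values and the bar.
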(fn ConstructionScript
  (|CallParentFunction))

(fn BPCalculateStarRating
  (params (IncomingStarRating :type Float%20%28double-precision%29) (Cash :type Integer))
  (Math|Integer|IncrementInt (Variables|Default|GetAmountofOrders)
    (:%20%20
      (if (== (Utilities|Array|Length (Variables|Default|GetPastRatings)) 0)
        (Variables|Default|SetStarRating (Math|Float|Max(Float) IncomingStarRating 0.0))
        (else
          (for _array_element (Variables|Default|GetPastRatings)
            (Variables|Default|SetSumOfRatings (+ _array_element (Variables|Default|GetSumOfRatings)))
            (Development|PrintString "Hello"))
          (if (and (>= (Variables|Default|GetStarRating) 4.9) (== IncomingStarRating 5.0))
            (Variables|Default|SetStarRating 5.0)
            (else
              (Variables|Default|SetStarRating (Math|Float|Max(Float) (/ (+ (Variables|Default|GetSumOfRatings) IncomingStarRating) (Variables|Default|GetAmountofOrders)) 0.0))))))
      (Utilities|Array|Add (Variables|Default|GetPastRatings) IncomingStarRating)
      (Development|PrintString (Utilities|String|ToString(Text) (Utilities|Text|FormatText "Reward is: {cash} & {starnumber}" Cash (Variables|Default|GetStarRating))))
      (Variables|Default|SetSumOfRatings 0.0)
      (bind _aswbp_order_screen_ui (Utilities|Casting|CastToWBP_OrderScreenUI (UserInterface|GetWidget (Variables|Default|GetWidget_0))))
      (Progress|SetPercent (Variables|/Game/UI/WBPs/CompoundCreator/WBP_StarRating.WBP_StarRating_C|GetProgressBar_138 (Variables|/Game/UI/WBPs/CompoundCreator/WBP_OrderScreenUI.WBP_OrderScreenUI_C|GetWBP_StarRating _aswbp_order_screen_ui)) (* (Variables|Default|GetStarRating) 0.2))
      (bind _structout (Utilities|Struct|SetmembersinRatingStruct (Variables|Default|GetRatingStruct) (Variables|Default|GetSumOfRatings) IncomingStarRating (Variables|Default|GetAmountofOrders) (Variables|Default|GetStarRating) (Variables|Default|GetPastRatings)))
      (Variables|Default|SetRatingStruct _structout)
      (bind _asbp_science_game_mode_comp_create (Utilities|Casting|CastToBP_ScienceGameModeCompCreate (Game|GetGameMode)))
      (Variables|/Game/BPs/CompoundCreator/BP_ScienceGameModeCompCreate.BP_ScienceGameModeCompCreate_C|SetCash _asbp_science_game_mode_comp_create (+ (Variables|/Game/BPs/CompoundCreator/BP_ScienceGameModeCompCreate.BP_ScienceGameModeCompCreate_C|GetCash _asbp_science_game_mode_comp_create) Cash)))))

(fn BPLoadValuesfromSave
  (bind _ratingstruct (Variables|Default|GetRatingStruct))
  (bind (_sumofratings _incomingstarrating _amountoforders _starrating _pastratings) (Utilities|Struct|BreakRatingStruct _ratingstruct))
  (Variables|Default|SetAmountofOrders _amountoforders)
  (Variables|Default|SetStarRating _starrating)
  (Variables|Default|SetPastRatings _pastratings)
  (bind _aswbp_order_screen_ui (Utilities|Casting|CastToWBP_OrderScreenUI (UserInterface|GetWidget (Variables|Default|GetWidget_0))))
  (Progress|SetPercent (Variables|/Game/UI/WBPs/CompoundCreator/WBP_StarRating.WBP_StarRating_C|GetProgressBar_138 (Variables|/Game/UI/WBPs/CompoundCreator/WBP_OrderScreenUI.WBP_OrderScreenUI_C|GetWBP_StarRating _aswbp_order_screen_ui)) (* (Variables|Default|GetStarRating) 0.2)))