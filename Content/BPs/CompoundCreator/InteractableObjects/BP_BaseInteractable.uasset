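; Base Blueprint for compound-creator interactables that unlock through a purchase widget, with no cost check in this graph.
; BeginPlay sets the tooltip, while DoStuff2 creates a dynamic material and checks the game mode's UnlockedInteractables.
; Locked objects bind the second widget's button to OnClickedBeaker, which adds the object to that list.
; Unlocked objects hide both widgets and switch the material's "bool" parameter on.
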(event Custom|OnClickedBeaker
  (Rendering|SetVisibility (Variables|Default|GetPurchaseWidget) false false)
  (Rendering|Material|SetScalarParameterValue (Variables|Default|GetDynamicMatRef) "bool" 1.0 :!class /Script/Engine.MaterialInstanceDynamic)
  (Variables|Default|SetbUnlocked true)
  (bind _asbp_science_game_mode_comp_create (Utilities|Casting|CastToBP_ScienceGameModeCompCreate (Game|GetGameMode)))
  (Utilities|Array|Add (Variables|/Game/BPs/CompoundCreator/BP_ScienceGameModeCompCreate.BP_ScienceGameModeCompCreate_C|GetUnlockedInteractables _asbp_science_game_mode_comp_create) self))

(event Custom|DoStuff2
  (bind _returnvalue (Rendering|Material|CreateDynamicMaterialInstance (Variables|Default|GetStaticMesh) 0 0 "None" :!class /Script/Engine.PrimitiveComponent))
  (Variables|Default|SetDynamicMatRef _returnvalue)
  (bind _asbp_science_game_mode_comp_create (Utilities|Casting|CastToBP_ScienceGameModeCompCreate (Game|GetGameMode)))
  (if (Utilities|Array|ContainsItem (Variables|/Game/BPs/CompoundCreator/BP_ScienceGameModeCompCreate.BP_ScienceGameModeCompCreate_C|GetUnlockedInteractables _asbp_science_game_mode_comp_create) self)
    (Rendering|SetVisibility (Variables|Default|GetPurchaseWidget) false false)
    (Variables|Default|SetbUnlocked true)
    (Rendering|Material|SetScalarParameterValue (Variables|Default|GetDynamicMatRef) "bool" 1.0 :!class /Script/Engine.MaterialInstanceDynamic)
    (else
      (bind _aswbp_purchase_widget_2 (Utilities|Casting|CastToWBP_PurchaseWidget2 (UserInterface|GetWidget (Variables|Default|GetPurchaseWidget2))))
      (EventDispatchers|BindEventtoOnClicked (Variables|/Game/UI/WBPs/CompoundCreator/WBP_PurchaseWidget2.WBP_PurchaseWidget2_C|GetButton_43 _aswbp_purchase_widget_2) (delegate Custom|OnClickedBeaker)))))

(event EventBeginPlay
  (bind _aswbp_purchase_widget (Utilities|Casting|CastToWBP_PurchaseWidget (UserInterface|GetWidget (Variables|Default|GetPurchaseWidget))))
  (Rendering|Components|TextRender|SetText (Variables|/Game/UI/WBPs/CompoundCreator/WBP_PurchaseWidget.WBP_PurchaseWidget_C|Gettooltiptextblock _aswbp_purchase_widget) (Variables|Default|GetPurchaseTooltipText)))

(fn ConstructionScript)