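; Wall calendar actor for the compound creator that tracks the in-game day and ends it when its End Day button is clicked.
; Past days appear as disabled buttons on the wall widget, restorable through SetupNextDay, and the week resets once the last day is reached.
; Ending a day advances the index, saves it with unlocked interactables and current orders to ScienceSaveGame, then shows a viewport calendar widget.
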(event Custom|ClickedExit
  (bind _nextdayindex (Variables|Default|GetNextDayIndex))
  (bind _returnvalue (SaveGame|DoesSaveGameExist "Test"))
  (if _returnvalue
    (if (not (Variables|Default|GetbIsAtEnd))
      (CallFunction|IterateCalendar)
      (CallFunction|CreateSaveSlotandSaveData :!label _label)
      (Utilities|IsValid (Variables|Default|GetCalendarWidgetRef)
        (:Is%20Valid
          (UserInterface|Viewport|AddtoViewport (Variables|Default|GetCalendarWidgetRef) 0))
        (:Is%20Not%20Valid
          (bind _returnvalue_2 (UserInterface|CreateWidget "/Game/UI/WBPs/CompoundCreator/WBP_CalendarCompCreator.WBP_CalendarCompCreator_C"))
          (bind _output_get (Variables|Default|SetCalendarWidgetRef _returnvalue_2))
          (if (== _nextdayindex 0)
            (for _array_element (Class|PanelWidget|GetAllChildren (Variables|/Game/UI/WBPs/CompoundCreator/WBP_CalendarCompCreator.WBP_CalendarCompCreator_C|GetDayImageHolder (Variables|Default|GetCalendarWidgetRef)))
              (Widget|SetIsEnabled _array_element true))
            (UserInterface|Viewport|AddtoViewport _output_get 0)
            (else
              (for _index (range 0 (- _nextdayindex 1))
                (Widget|SetIsEnabled (Utilities|Array|Get(acopy) (Class|PanelWidget|GetAllChildren (Variables|/Game/UI/WBPs/CompoundCreator/WBP_CalendarCompCreator.WBP_CalendarCompCreator_C|GetDayImageHolder (Variables|Default|GetCalendarWidgetRef))) _index) false))
              (UserInterface|Viewport|AddtoViewport _output_get 0))))))
    (else
      (CallFunction|SetMondayDisabled)
      (bind _aswbp_calendar_comp_creator_wall (Utilities|Casting|CastToWBP_CalendarCompCreatorWall (UserInterface|GetWidget (Variables|Default|GetWidget_0))))
      (Variables|Default|SetNextDayButton (Variables|/Game/UI/WBPs/CompoundCreator/WBP_CalendarCompCreatorWall.WBP_CalendarCompCreatorWall_C|GetTuesdayButton _aswbp_calendar_comp_creator_wall))
      (goto _label))))

(event Custom|SetupNextDay
  (params (NewParam :type Integer))
  (bind _output_get (Variables|Default|SetNextDayIndex NewParam))
  (if (== _output_get 0)
    (bind _aswbp_calendar_comp_creator_wall (Utilities|Casting|CastToWBP_CalendarCompCreatorWall (UserInterface|GetWidget (Variables|Default|GetWidget_0))))
    (Widget|SetIsEnabled (Variables|/Game/UI/WBPs/CompoundCreator/WBP_CalendarCompCreatorWall.WBP_CalendarCompCreatorWall_C|GetSundayButton _aswbp_calendar_comp_creator_wall) true)
    (Variables|Default|SetbShouldIncre false)
    (else
      (bind _aswbp_calendar_comp_creator_wall_2 (Utilities|Casting|CastToWBP_CalendarCompCreatorWall (UserInterface|GetWidget (Variables|Default|GetWidget_0))))
      (if (== (Variables|Default|GetNextDayIndex) 1)
        (bind _aswbp_calendar_comp_creator_wall_3 (Utilities|Casting|CastToWBP_CalendarCompCreatorWall (UserInterface|GetWidget (Variables|Default|GetWidget_0))))
        (Widget|SetIsEnabled (Variables|/Game/UI/WBPs/CompoundCreator/WBP_CalendarCompCreatorWall.WBP_CalendarCompCreatorWall_C|GetSundayButton _aswbp_calendar_comp_creator_wall_3) false)
        (else
          (for _index (range 0 (- (Variables|Default|GetNextDayIndex) 1))
            (Widget|SetIsEnabled (Utilities|Array|Get(acopy) (Class|PanelWidget|GetAllChildren (Variables|/Game/UI/WBPs/CompoundCreator/WBP_CalendarCompCreatorWall.WBP_CalendarCompCreatorWall_C|GetDayImageHolder _aswbp_calendar_comp_creator_wall_2)) _index) false)))))))

(event EventBeginPlay
  (bind _aswbp_calendar_comp_creator_wall (Utilities|Casting|CastToWBP_CalendarCompCreatorWall (UserInterface|GetWidget (Variables|Default|GetWidget_0))))
  (EventDispatchers|BindEventtoOnClicked (Variables|/Game/UI/WBPs/CompoundCreator/WBP_CalendarCompCreatorWall.WBP_CalendarCompCreatorWall_C|GetEndDay _aswbp_calendar_comp_creator_wall) (delegate Custom|ClickedExit)))

(fn ConstructionScript)

(fn BPSetNextDayDisabled
  (params (NextDayButton :type Integer))
  (bind _aswbp_calendar_comp_creator_wall (Utilities|Casting|CastToWBP_CalendarCompCreatorWall (UserInterface|GetWidget (Variables|Default|GetWidget_0))))
  (Widget|SetIsEnabled (Utilities|Array|Get(acopy) (Class|PanelWidget|GetAllChildren (Variables|/Game/UI/WBPs/CompoundCreator/WBP_CalendarCompCreatorWall.WBP_CalendarCompCreatorWall_C|GetDayImageHolder _aswbp_calendar_comp_creator_wall)) NextDayButton) false))

(fn BPSetMondayDisabled
  (bind _aswbp_calendar_comp_creator_wall (Utilities|Casting|CastToWBP_CalendarCompCreatorWall (UserInterface|GetWidget (Variables|Default|GetWidget_0))))
  (Widget|SetIsEnabled (Variables|/Game/UI/WBPs/CompoundCreator/WBP_CalendarCompCreatorWall.WBP_CalendarCompCreatorWall_C|GetMondayButton _aswbp_calendar_comp_creator_wall) false))

(fn BPSetNextDayDisabled2
  (params (NextDayButton :type Button%20Object%20Reference)))

(fn BPResetCalendar
  (Variables|Default|SetbIsAtEnd true)
  (bind _aswbp_calendar_comp_creator_wall (Utilities|Casting|CastToWBP_CalendarCompCreatorWall (UserInterface|GetWidget (Variables|Default|GetWidget_0))))
  (for _array_element (Class|PanelWidget|GetAllChildren (Variables|/Game/UI/WBPs/CompoundCreator/WBP_CalendarCompCreatorWall.WBP_CalendarCompCreatorWall_C|GetDayImageHolder _aswbp_calendar_comp_creator_wall))
    (Widget|SetIsEnabled _array_element true)
    (Variables|Default|SetNextDayIndex 0)
    (Variables|Default|SetbShouldIncre false)))

(fn BPSaveandDisable
  (Utilities|IsValid (Variables|Default|GetAs%20Science%20Save%20Game)
    (:Is%20Valid
      _)
    (:Is%20Not%20Valid
      (bind _returnvalue (SaveGame|CreateSaveGameObject "/Game/BPs/CompoundCreator/ScienceSaveGame.ScienceSaveGame_C"))
      (bind _output_get (Variables|Default|SetAs%20Science%20Save%20Game _returnvalue))))
  (Variables|/Game/BPs/CompoundCreator/ScienceSaveGame.ScienceSaveGame_C|SetUnlockedInteractables _output_get (Variables|Default|GetUnlockedInteractables))
  (Variables|/Game/BPs/CompoundCreator/ScienceSaveGame.ScienceSaveGame_C|SetNextDayIndex _output_get (Variables|Default|GetNextDayIndex))
  (SaveGame|SaveGametoSlot (Variables|Default|GetAs%20Science%20Save%20Game) "Test")
  (Development|PrintString (Utilities|String|ToString(Integer) (Variables|Default|GetNextDayIndex))))

(fn BPSaveandDisableNoIncr
  (CallFunction|SetNextDayDisabled (Variables|Default|GetNextDayIndex))
  (Utilities|IsValid (Variables|Default|GetAs%20Science%20Save%20Game)
    (:Is%20Valid
      _)
    (:Is%20Not%20Valid
      (bind _returnvalue (SaveGame|CreateSaveGameObject "/Game/BPs/CompoundCreator/ScienceSaveGame.ScienceSaveGame_C"))
      (bind _output_get (Variables|Default|SetAs%20Science%20Save%20Game _returnvalue))))
  (Variables|/Game/BPs/CompoundCreator/ScienceSaveGame.ScienceSaveGame_C|SetUnlockedInteractables _output_get (Variables|Default|GetUnlockedInteractables))
  (Variables|/Game/BPs/CompoundCreator/ScienceSaveGame.ScienceSaveGame_C|SetNextDayIndex _output_get (Variables|Default|GetNextDayIndex))
  (SaveGame|SaveGametoSlot (Variables|Default|GetAs%20Science%20Save%20Game) "Test")
  (Development|PrintString (Utilities|String|ToString(Integer) (Variables|Default|GetNextDayIndex)))
  (Game|OpenLevel(byName) "ChemistryScreen"))

(fn BPCreateSaveSlotandSaveData
  ;[1 1 1] Fill array with all unlocked interactables
  (bind _outactors (Actor|GetAllActorsOfClass "/Game/BPs/CompoundCreator/InteractableObjects/BP_BaseInteractable.BP_BaseInteractable_C"))
  (for _array_element _outactors
    (if (Variables|/Game/BPs/CompoundCreator/InteractableObjects/BP_BaseInteractable.BP_BaseInteractable_C|GetbUnlocked _array_element)
      (Utilities|Array|AddUnique (Variables|Default|GetUnlockedInteractables) _array_element)))
  ;[1 1 1] create save game object
  (Utilities|IsValid (Variables|Default|GetAs%20Science%20Save%20Game)
    (:Is%20Valid
      _)
    (:Is%20Not%20Valid
      (bind _returnvalue (SaveGame|CreateSaveGameObject "/Game/BPs/CompoundCreator/ScienceSaveGame.ScienceSaveGame_C"))
      (bind _output_get (Variables|Default|SetAs%20Science%20Save%20Game _returnvalue))))
  ;[1 1 1] save unlocked interactable
  (Variables|/Game/BPs/CompoundCreator/ScienceSaveGame.ScienceSaveGame_C|SetUnlockedInteractables _output_get (Variables|Default|GetUnlockedInteractables))
  ;[1 1 1] save calendar data
  (if (Variables|Default|GetbShouldIncre)
    (Math|Integer|IncrementInt (Variables|Default|GetNextDayIndex)
      (:%20%20
        _))
    (else
      (Variables|Default|SetNextDayIndex 0)))
  (Variables|/Game/BPs/CompoundCreator/ScienceSaveGame.ScienceSaveGame_C|SetNextDayIndex _output_get (Variables|Default|GetNextDayIndex))
  ;[1 1 1] save current orders
  (bind _returnvalue_2 (Actor|GetActorOfClass "/Game/BPs/CompoundCreator/BP_OrderScreen.BP_OrderScreen_C"))
  (bind _aswbp_order_screen_ui (Utilities|Casting|CastToWBP_OrderScreenUI (UserInterface|GetWidget (Variables|/Game/BPs/CompoundCreator/BP_OrderScreen.BP_OrderScreen_C|GetWidget_0 _returnvalue_2))))
  (for _array_element_2 (Class|PanelWidget|GetAllChildren (Variables|/Game/UI/WBPs/CompoundCreator/WBP_OrderScreenUI.WBP_OrderScreenUI_C|GetLeftScrollBoxCurrent _aswbp_order_screen_ui))
    (bind _aswbp_order_entry_current (Utilities|Casting|CastToWBP_OrderEntryCurrent _array_element_2))
    (Utilities|Array|Add (Variables|/Game/BPs/CompoundCreator/ScienceSaveGame.ScienceSaveGame_C|GetCurrentOrders _output_get) (Variables|/Game/UI/WBPs/CompoundCreator/WBP_OrderEntryCurrent.WBP_OrderEntryCurrent_C|GetOrderData _aswbp_order_entry_current)))
  ;[1 1 1] Save the actual Slot
  (SaveGame|SaveGametoSlot (Variables|Default|GetAs%20Science%20Save%20Game) "Test")
  (Development|PrintString (Utilities|String|ToString(Integer) (Variables|Default|GetNextDayIndex))))

(fn BPIterateCalendar
  (bind _aswbp_calendar_comp_creator_wall (Utilities|Casting|CastToWBP_CalendarCompCreatorWall (UserInterface|GetWidget (Variables|Default|GetWidget_0))))
  (bind (_array_element _array_index) (Utilities|Array|ForEachLoopwithBreak (Class|PanelWidget|GetAllChildren (Variables|/Game/UI/WBPs/CompoundCreator/WBP_CalendarCompCreatorWall.WBP_CalendarCompCreatorWall_C|GetDayImageHolder _aswbp_calendar_comp_creator_wall)) :!label _label)
    (:LoopBody
      (bind _asbutton (Utilities|Casting|CastToButton _array_element))
      (if (Class|Widget|GetIsEnabled _asbutton)
        (goto _label Break)
        (elif (== _array_index 5)
          (CallFunction|ResetCalendar))))
    (:Completed
      (if (Variables|Default|GetbIsAtEnd)
        (Variables|Default|SetbIsAtEnd false)
        (Variables|Default|SetNextDayIndex 0)
        (Variables|Default|SetbShouldIncre false)
        (else
          (CallFunction|SaveandDisable)
          (Variables|Default|SetbShouldIncre true))))))