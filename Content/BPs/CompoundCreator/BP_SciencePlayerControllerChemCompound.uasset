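; Player controller for the chemistry compound-creator, handling camera zoom, interaction with lab objects and the pause menu.
; The mouse wheel blends between primary, secondary and per-object tertiary cameras unless the inventory is open.
; Clicking an interactable's mesh opens a menu: Mix matches its inventory against compound DataTable recipes, yielding a compound or "Unknown", and Clear empties it.
; Move lists other unlocked interactables in a combo box, but its selection handler is empty.
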(event Custom|MoveButtonClicked
  (bind _returnvalue (Game|GetPlayerController 0))
  (bind (_locationx _locationy) (Game|Player|GetMousePosition _returnvalue))
  ;[1 1 1] create interactionmenu
  (bind _comboboxref (Variables|Default|GetComboBoxRef)
    (:then
      (Widget|RemovefromParent _comboboxref))
    (:else
      _))
  (bind _returnvalue_2 (UserInterface|CreateWidget "/Game/UI/WBPs/CompoundCreator/WBP_InteractionMenuMoveCombobox.WBP_InteractionMenuMoveCombobox_C"))
  (bind _output_get (Variables|Default|SetComboBoxRef _returnvalue_2))
  (Variables|/Game/UI/WBPs/CompoundCreator/WBP_InteractionMenuMoveCombobox.WBP_InteractionMenuMoveCombobox_C|SetFromObj _output_get (Variables|Default|GetInteractableObject))
  (UserInterface|Viewport|AddtoViewport _output_get 0)
  (Class|UserWidget|SetPositioninViewport _output_get (Math|Vector2D|MakeVector2D _locationx _locationy) true)
  (EventDispatchers|BindEventtoOnSelectionChanged (Variables|/Game/UI/WBPs/CompoundCreator/WBP_InteractionMenuMoveCombobox.WBP_InteractionMenuMoveCombobox_C|GetComboBoxKey_188 _output_get) (delegate Custom|SelectionChangedMoveto))
  (EventDispatchers|BindEventtoOnOpening (Variables|/Game/UI/WBPs/CompoundCreator/WBP_InteractionMenuMoveCombobox.WBP_InteractionMenuMoveCombobox_C|GetComboBoxKey_188 _output_get) (delegate Custom|CustomEvent_0)))

(event Custom|SelectionChangedMoveto
  (params (SelectedItem :type Name) (SelectionType :type ESelectInfo%20Enum :default "OnKeyPress"))
  ;[1 1 1] move to combobox
)

(event Custom|ClickedMix
  (bind _recipestruct (Variables|Default|GetRecipeStruct))
  (bind _interactableobject (Variables|Default|GetInteractableObject))
  (bind _interactableobject_2 (Variables|Default|GetInteractableObject))
  (bind _recipestruct_2 (Variables|Default|GetRecipeStruct))
  (bind _interactableobject_3 (Variables|Default|GetInteractableObject))
  (bind _bp_inventorycomponent (Variables|/Game/BPs/CompoundCreator/InteractableObjects/BP_BaseInteractable.BP_BaseInteractable_C|GetBP_InventoryComponent _interactableobject))
  (bind _bp_inventorycomponent_2 (Variables|/Game/BPs/CompoundCreator/InteractableObjects/BP_BaseInteractable.BP_BaseInteractable_C|GetBP_InventoryComponent _interactableobject_3))
  (bind _bp_inventorycomponent_3 (Variables|/Game/BPs/CompoundCreator/InteractableObjects/BP_BaseInteractable.BP_BaseInteractable_C|GetBP_InventoryComponent _interactableobject_2))
  (bind _inventorycontent (Variables|/Game/Data/CompoundCreator/Inventory/BP_InventoryComponent.BP_InventoryComponent_C|GetInventoryContent _bp_inventorycomponent))
  ;[1 1 1] loop through all possible compounds
  (if (> (Utilities|Map|Length (Variables|/Game/Data/CompoundCreator/Inventory/BP_InventoryComponent.BP_InventoryComponent_C|GetInventoryContent (Variables|/Game/BPs/CompoundCreator/InteractableObjects/BP_BaseInteractable.BP_BaseInteractable_C|GetBP_InventoryComponent (Variables|Default|GetInteractableObject)))) 0)
    (bind _outrownames (DataTable|GetDataTableRowNames "/Game/Data/CompoundCreator/Inventory/ItemDataTableCompound.ItemDataTableCompound"))
    (for _array_element _outrownames
      (bind _returnvalue (Utilities|GetDataTableRow "/Game/Data/CompoundCreator/Inventory/ItemDataTableCompound.ItemDataTableCompound" _array_element)
        (:then
          ;[1 1 1] see if the interactable objects inventory has the right stuff to make a compound
          (bind (_array_element_2 _array_index) (Utilities|Array|ForEachLoopwithBreak (.ElementList (Utilities|Struct|BreakItemStructCompound _returnvalue)))
            (:LoopBody
              (if (Math|Boolean|ANDBoolean (== (Utilities|Map|Length _inventorycontent) (Utilities|Array|Length (.ElementList (Utilities|Struct|BreakItemStructCompound _returnvalue)))) (Utilities|Map|Contains _inventorycontent (.Name (Utilities|Struct|BreakRecipeStruct _array_element_2))) (== (.Value (Utilities|Map|Find _inventorycontent (.Name (Utilities|Struct|BreakRecipeStruct _array_element_2)))) (.Quantity (Utilities|Struct|BreakRecipeStruct _array_element_2))))
                (Utilities|Array|Add _recipestruct_2 _array_element_2)
                (Utilities|Struct|SetmembersinRecipeStruct (Utilities|Array|Get(acopy) _recipestruct_2 _array_index) true)
                (Variables|Default|SetbIsUnknown false)
                (else
                  (Utilities|Map|Clear (Variables|/Game/Data/CompoundCreator/Inventory/BP_InventoryComponent.BP_InventoryComponent_C|GetInventoryContent _bp_inventorycomponent_3))
                  (Default|AddtoInventory _bp_inventorycomponent_3 "Unknown" 1)
                  (bind _asbp_starter_beaker (Utilities|Casting|CastToBP_StarterBeaker _interactableobject_2))
                  (Default|ClearFluidText _asbp_starter_beaker)
                  (Default|UpdateFluidLevel _asbp_starter_beaker "Unknown")
                  (Variables|Default|SetbIsUnknown true))))
            (:Completed
              ;[1 1 1] should we make a compound
              (if (== (Utilities|Array|Length (.ElementList (Utilities|Struct|BreakItemStructCompound _returnvalue))) (Utilities|Array|Length _recipestruct))
                (bind _array_element_3 (Utilities|Array|ForEachLoopwithBreak _recipestruct :!label _label)
                  (:LoopBody
                    (if (.bFufilled (Utilities|Struct|BreakRecipeStruct _array_element_3))
                      (Variables|Default|SetbShouldMake true)
                      (else
                        (Variables|Default|SetbShouldMake false)
                        (goto _label Break))))
                  (:Completed
                    (if (Variables|Default|GetbShouldMake)
                      ;[1 1 1] remove ingredients and add the compound
                      (if (not (Variables|Default|GetbIsUnknown))
                        (Utilities|Map|Clear (Variables|/Game/Data/CompoundCreator/Inventory/BP_InventoryComponent.BP_InventoryComponent_C|GetInventoryContent _bp_inventorycomponent_2))
                        (Default|AddtoInventory _bp_inventorycomponent_2 (Utilities|String|StringToName (.Name (Utilities|Struct|BreakItemStructCompound _returnvalue))) 1)
                        (bind _asbp_starter_beaker_2 (Utilities|Casting|CastToBP_StarterBeaker _interactableobject_3))
                        (Default|ClearFluidText _asbp_starter_beaker_2)
                        (Default|UpdateFluidLevel _asbp_starter_beaker_2 (Utilities|String|StringToName (.Name (Utilities|Struct|BreakItemStructCompound _returnvalue))))))))))))))))

(event Custom|ClearClicked
  ;[1 1 1] Clear the interactable items inventory
  (Utilities|Map|Clear (Variables|/Game/Data/CompoundCreator/Inventory/BP_InventoryComponent.BP_InventoryComponent_C|GetInventoryContent (Variables|/Game/BPs/CompoundCreator/InteractableObjects/BP_BaseInteractable.BP_BaseInteractable_C|GetBP_InventoryComponent (Variables|Default|GetInteractableObject))))
  (bind _asbp_starter_beaker (Utilities|Casting|CastToBP_StarterBeaker (Variables|Default|GetInteractableObject)))
  (Default|ClearFluidText _asbp_starter_beaker)
  (Default|UpdateFluidLevel _asbp_starter_beaker "None"))

(event Custom|CustomEvent_0
  (bind _comboboxref (Variables|Default|GetComboBoxRef))
  ;[1 1 1] setting up move to combobox
  (bind _outactors (Actor|GetAllActorsOfClass "/Game/BPs/CompoundCreator/InteractableObjects/BP_BaseInteractable.BP_BaseInteractable_C"))
  (for _array_element _outactors
    (if (and (Variables|/Game/BPs/CompoundCreator/InteractableObjects/BP_BaseInteractable.BP_BaseInteractable_C|GetbUnlocked _array_element) (!= (Variables|/Game/BPs/CompoundCreator/InteractableObjects/BP_BaseInteractable.BP_BaseInteractable_C|GetName (Variables|Default|GetInteractableObject)) (Variables|/Game/BPs/CompoundCreator/InteractableObjects/BP_BaseInteractable.BP_BaseInteractable_C|GetName _array_element)))
      (Default|OnGenerateItemWidget0 _comboboxref (Variables|/Game/BPs/CompoundCreator/InteractableObjects/BP_BaseInteractable.BP_BaseInteractable_C|GetName _array_element))
      (Default|OnGenerateContentWidget0 _comboboxref (Variables|/Game/BPs/CompoundCreator/InteractableObjects/BP_BaseInteractable.BP_BaseInteractable_C|GetName _array_element))
      (Class|ComboBoxKey|AddOption (Variables|/Game/UI/WBPs/CompoundCreator/WBP_InteractionMenuMoveCombobox.WBP_InteractionMenuMoveCombobox_C|GetComboBoxKey_188 (stale Custom|MoveButtonClicked _output_get)) (Variables|/Game/BPs/CompoundCreator/InteractableObjects/BP_BaseInteractable.BP_BaseInteractable_C|GetName _array_element)))))

(event Input|KeyboardEvents|Tab
  (params (Key :type Key%20Structure :default "None"))
  (:Pressed
    (Utilities|FlowControl|FlipFlop
      (:A
        (bind _pausemenuref (Variables|Default|GetPauseMenuRef)
          (:then
            (UserInterface|Viewport|AddtoViewport _pausemenuref 0))
          (:else
            (bind _returnvalue (UserInterface|CreateWidget "/Game/UI/WBPs/Main/WBP_Pause.WBP_Pause_C"))
            (bind _output_get (Variables|Default|SetPauseMenuRef _returnvalue))
            (UserInterface|Viewport|AddtoViewport _output_get 0)
            (Variables|/Script/Engine.PlayerController|SetbShowMouseCursor (Game|GetPlayerController 0) true))))
      (:B
        (bind _pausemenuref_2 (Variables|Default|GetPauseMenuRef)
          (:then
            (Widget|RemovefromParent _pausemenuref_2))
          (:else))))))

(event Input|MouseEvents|LeftMouseButton
  (params (Key :type Key%20Structure :default "None"))
  (bind _returnvalue (Game|GetPlayerController 0))
  (bind (_locationx _locationy) (Game|Player|GetMousePosition))
  (bind (_hitresult _returnvalue_2) (Game|Player|GetHitResultUnderCursorbyChannel _returnvalue "TraceTypeQuery1" true))
  (bind (_bblockinghit _binitialoverlap _time _distance _location _impactpoint _normal _impactnormal _physmat _hitactor _hitcomponent) (Collision|BreakHitResult _hitresult))
  ;[1 1 1] create interactionmenu
  (:Pressed
    (if _returnvalue_2
      (bind _asbp_base_interactable (Utilities|Casting|CastToBP_BaseInteractable _hitactor)
        (:then
          (Variables|Default|SetInteractableObject _asbp_base_interactable)
          (if (== (Variables|/Game/BPs/CompoundCreator/InteractableObjects/BP_BaseInteractable.BP_BaseInteractable_C|GetStaticMesh _asbp_base_interactable) _hitcomponent)
            (bind _interactionmenuref (Variables|Default|GetInteractionMenuRef)
              (:then
                (Widget|RemovefromParent _interactionmenuref))
              (:else
                _))
            (bind _comboboxref (Variables|Default|GetComboBoxRef)
              (:then
                (Widget|RemovefromParent _comboboxref))
              (:else
                _))
            (bind _returnvalue_3 (UserInterface|CreateWidget "/Game/UI/WBPs/CompoundCreator/WBP_InteractionMenu.WBP_InteractionMenu_C"))
            (bind _output_get (Variables|Default|SetInteractionMenuRef _returnvalue_3))
            (UserInterface|Viewport|AddtoViewport _returnvalue_3 0)
            (Class|UserWidget|SetPositioninViewport _returnvalue_3 (Math|Vector2D|MakeVector2D _locationx _locationy) true)
            (UserInterface|Animation|PlayAnimation _output_get (Variables|/Game/UI/WBPs/CompoundCreator/WBP_InteractionMenu.WBP_InteractionMenu_C|GetExpand _returnvalue_3) 0.0 1 "Forward" 1.0 false)
            (EventDispatchers|BindEventtoOnClicked (Variables|/Game/UI/WBPs/CompoundCreator/WBP_InteractionMenu.WBP_InteractionMenu_C|GetMoveToButton _output_get) (delegate Custom|MoveButtonClicked))
            (EventDispatchers|BindEventtoOnClicked (Variables|/Game/UI/WBPs/CompoundCreator/WBP_InteractionMenu.WBP_InteractionMenu_C|GetMixButton _output_get) (delegate Custom|ClickedMix))
            ;[1 1 1] Clear the interactable items inventory
            (EventDispatchers|BindEventtoOnClicked (Variables|/Game/UI/WBPs/CompoundCreator/WBP_InteractionMenu.WBP_InteractionMenu_C|GetClearButton _output_get) (delegate Custom|ClearClicked))))
        (:CastFailed
          (bind _interactionmenuref_2 (Variables|Default|GetInteractionMenuRef)
            (:then
              (Widget|RemovefromParent _interactionmenuref_2))
            (:else
              _))
          (bind _comboboxref_2 (Variables|Default|GetComboBoxRef)
            (:then
              (Widget|RemovefromParent _comboboxref_2))
            (:else)))))))

(event Input|MouseEvents|MouseWheelUp
  (params (Key :type Key%20Structure :default "None"))
  (bind _returnvalue (Game|GetPlayerController 0))
  (bind _array (Utilities|Array|MakeArray "ObjectTypeQuery1" "ObjectTypeQuery2" "ObjectTypeQuery3" "ObjectTypeQuery4" "ObjectTypeQuery5" "ObjectTypeQuery6"))
  (bind (_hitresult _returnvalue_2) (Class|PlayerController|GetHitResultUnderCursorforObjects _returnvalue _array true))
  ;[1 1 1] Change zoom
  (:Pressed
    (bind _open_ (CallFunction|CheckInventoryOpen))
    (if (and (not _open_) _returnvalue_2)
      (if (Variables|Default|GetbPrimary)
        (CallFunction|SetSecondaryView)
        (elif (Variables|Default|GetbSecondary)
          (CallFunction|SetTertiaryView (.HitActor (Collision|BreakHitResult _hitresult))))))))

(event Input|MouseEvents|MouseWheelDown
  (params (Key :type Key%20Structure :default "None"))
  ;[1 1 1] Change zoom
  (:Pressed
    (bind _open_ (CallFunction|CheckInventoryOpen))
    (if (and (not _open_) (Variables|Default|GetbTertiary))
      (CallFunction|SetSecondaryView)
      (elif (Variables|Default|GetbSecondary)
        (CallFunction|SetPrimaryView)))))

(event Input|KeyboardEvents|LeftAlt
  (params (Key :type Key%20Structure :default "None"))
  (:Pressed
    (bind _isa (Utilities|FlowControl|FlipFlop)
      (:A
        (Variables|Default|SetbShowMouseCursor _isa))
      (:B
        (Variables|Default|SetbShowMouseCursor _isa)))))

(fn ConstructionScript)

(fn BPSetSecondaryView
  (Game|Player|SetViewTargetwithBlend self 0.5 "VTBlend_Linear" 0.0 true)
  (Variables|Default|SetbTertiary false)
  (Variables|Default|SetbSecondary true)
  (Variables|Default|SetbPrimary false)
  (bind _outactors (Actor|GetAllActorsOfClass "/Game/BPs/CompoundCreator/InteractableObjects/BP_BaseInteractable.BP_BaseInteractable_C"))
  (for _array_element _outactors
    (Variables|/Game/BPs/CompoundCreator/InteractableObjects/BP_BaseInteractable.BP_BaseInteractable_C|SetbSelected _array_element false)))

(fn BPSetTertiaryView
  (params (Object :type Object%20Object%20Reference))
  (Variables|Default|SetTertiaryObject Object)
  (bind _asbp_base_interactable (Utilities|Casting|CastToBP_BaseInteractable (Variables|Default|GetTertiaryObject)))
  (Variables|/Game/BPs/CompoundCreator/InteractableObjects/BP_BaseInteractable.BP_BaseInteractable_C|SetbSelected _asbp_base_interactable true)
  (Game|Player|SetViewTargetwithBlend (Variables|/Script/Engine.ChildActorComponent|GetChildActor (Variables|/Game/BPs/CompoundCreator/InteractableObjects/BP_BaseInteractable.BP_BaseInteractable_C|GetBP_cameraActor _asbp_base_interactable)) 0.5 "VTBlend_Linear" 0.0 true)
  (Variables|Default|SetbTertiary true)
  (Variables|Default|SetbSecondary false)
  (Variables|Default|SetbPrimary false))

(fn BPSetPrimaryView
  (bind _returnvalue (Actor|GetActorOfClass "/Game/BPs/CompoundCreator/BP_cameraActorPrimary.BP_cameraActorPrimary_C"))
  (Game|Player|SetViewTargetwithBlend _returnvalue 0.5 "VTBlend_Linear" 0.0 true)
  (Variables|Default|SetbTertiary false)
  (Variables|Default|SetbSecondary false)
  (Variables|Default|SetbPrimary true))

(fn BPCheckInventoryOpen
  (bind _asbp_chem_compound_hud (Utilities|Casting|CastToBP_ChemCompoundHUD (HUD|GetHUD)))
  (return (Variables|/Game/UI/WBPs/CompoundCreator/WBP_HUDCompoundCreator.WBP_HUDCompoundCreator_C|GetbInventoryOpen (Variables|/Game/BPs/CompoundCreator/BP_ChemCompoundHUD.BP_ChemCompoundHUD_C|GetHudWidgetRef _asbp_chem_compound_hud))))